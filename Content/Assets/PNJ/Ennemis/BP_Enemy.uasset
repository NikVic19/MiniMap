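; Enemy actor that moves its capsule between its spawn position and an offset set by Déplacement, then destroys itself after a short lifetime.
; BeginPlay stores the start location, starts the Movement event and destroys the actor after a fixed delay.
; Movement runs a timed MoveComponentTo, flips the target with a FlipFlop and calls itself to loop.
; The first move targets the start position, so displacement begins on the following move.
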(event `self.ReceiveBeginPlay`
  (bind _output_get (set `self.Startposition` (`SceneComponent.K2_GetComponentLocation` (`self.CapsuleComponent`))))
  (set `self.Target` _output_get)
  (`self.Movement`)
  (`KismetSystemLibrary.Delay` 4.0)
  (`self.K2_DestroyActor`))

(event `Movement`
  (bind _startposition (`self.Startposition`))
  (`KismetSystemLibrary.MoveComponentTo` (`self.CapsuleComponent`) (`self.Target`) (struct) false false 2.0)
  (`/Engine/EditorBlueprintResources/StandardMacros.FlipFlop`
    (:`A`
      (set `self.Target` (+ (`self.Déplacement`) _startposition)))
    (:`B`
      (set `self.Target` _startposition)))
  (`self.Movement`))

(fn `UserConstructionScript`)