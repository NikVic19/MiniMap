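; BP_MiniMap drives the player minimap, creating the WG_MiniMap widget and adding it to the viewport on BeginPlay.
; Each Tick it writes the player character's location and yaw, normalized to a 0–1 turn, into the MP_MiniMap Material Parameter Collection.
; UpdateIconPosition forwards a given position to the widget to move an icon.
; Tick also prints the player location as debug output.
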(event `self.ReceiveBeginPlay`
  (bind _returnvalue (`|GenericCreateObject` "/Game/Assets/MiniMap/WG_MiniMap.WG_MiniMap_C"))
  (`UserWidget.AddToViewport` _returnvalue 0)
  (set `self.WG Minimap` _returnvalue))

(event `self.ReceiveTick`
  (params (DeltaSeconds :type "Float (single-precision)"))
  (bind _returnvalue (`self.K2_GetActorLocation` (`GameplayStatics.GetPlayerCharacter` 0)))
  (`KismetSystemLibrary.PrintString` (`KismetStringLibrary.Conv_VectorToString` _returnvalue))
  (`KismetMaterialLibrary.SetVectorParameterValue` "/Game/Assets/MiniMap/MP_MiniMap.MP_MiniMap" "PlayerLocation" (`KismetMathLibrary.Conv_VectorToLinearColor` _returnvalue))
  (bind _yaw (`self.ComputeNormalizedYaw`))
  (`KismetMaterialLibrary.SetScalarParameterValue` "/Game/Assets/MiniMap/MP_MiniMap.MP_MiniMap" "Player Yaw" _yaw))

(event `/Game/Assets/MiniMap/BPI_MiniMap.UpdateIconPosition`
  (params (Position :type "Vector2D Structure"))
  (`/Game/Assets/MiniMap/WG_MiniMap.UpdateIconLocation` (`self.WG Minimap`) Position))

(fn `ComputeNormalizedYaw`
  (returns (Yaw :type "Float (double-precision)"))
  (bind _yaw (.yaw (`self.K2_GetActorRotation` (`GameplayStatics.GetPlayerCharacter` 0))))
  (if (> _yaw 0.0)
    (return (/ _yaw 360.0))
    (else
      (return (/ (+ _yaw 360.0) 360.0)))))

(fn `UserConstructionScript`)